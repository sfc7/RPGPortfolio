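; BP_PlayerCharacter_Fighter is the Fighter player character Blueprint, containing only debug shortcuts in its own graphs.
; The J debug key opens the Town level.
; The T debug key builds test stacks of gold, wood materials and HP potions through the item manager and adds them to the player's inventory component.
; BeginPlay, overlap, Tick and the construction script contain no logic.
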(event EventBeginPlay)

(event Collision|EventActorBeginOverlap
  (params (OtherActor :type Actor%20Object%20Reference)))

(event EventTick
  (params (DeltaSeconds :type Float%20%28single-precision%29)))

(event Input|KeyboardEvents|DebugKeyT
  (params (Key :type Key%20Structure :default "None") (ActionValue :type Input%20Action%20Value%20Structure))
  (:Pressed
    (for _array_element (Utilities|Array|MakeArray (Class|ItemManager|MakeItemtoAdd (Subsystems|GetItemManager) "/Game/MyProject/Data/Item/DA_Item_GoldBar.DA_Item_GoldBar" 50) (Class|ItemManager|MakeItemtoAdd (Subsystems|GetItemManager) "/Game/MyProject/Data/Item/DA_Item_ReinforcedWood.DA_Item_ReinforcedWood" 180) (Class|ItemManager|MakeItemtoAdd (Subsystems|GetItemManager) "/Game/MyProject/Data/Item/DA_Item_Wood.DA_Item_Wood" 190) (Class|ItemManager|MakeItemtoAdd (Subsystems|GetItemManager) "/Game/MyProject/Data/Item/DA_Item_HpPotion30.DA_Item_HpPotion30" 5) (Class|ItemManager|MakeItemtoAdd (Subsystems|GetItemManager) "/Game/MyProject/Data/Item/DA_Item_HpPotion50.DA_Item_HpPotion50" 190))
      (Class|PlayerInventoryComponent|AddItem (Variables|Default|GetPlayerItemInventoryComponent) _array_element))))

(event Input|KeyboardEvents|DebugKeyJ
  (params (Key :type Key%20Structure :default "None") (ActionValue :type Input%20Action%20Value%20Structure))
  (:Pressed
    (Game|OpenLevel(byName) "Town")))

(fn ConstructionScript)